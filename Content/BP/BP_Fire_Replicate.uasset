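; BP_Fire_Replicate is a fire actor that burns for a countdown and then switches off, demonstrating variable replication.
; On BeginPlay only the authority starts a looping one-second timer, which decrements CountdownTimer and then sets Deactivate once it runs out.
; The Deactivate RepNotify turns off the PFire effect, while Tick writes the remaining count to a text render.
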(event Custom|UpdateTimer
  (if (> (Variables|Default|GetCountdownTimer) 0)
    (Variables|Default|SetCountdownTimer (- (Variables|Default|GetCountdownTimer) 1))
    (else
      (Variables|Default|SetDeactivate true))))

(event EventBeginPlay
  (Networking|SwitchHasAuthority
    (:Authority
      (Utilities|Time|SetTimerbyEvent (delegate Custom|UpdateTimer) 1.0 true))))

(event EventTick
  (params (DeltaSeconds :type Float%20%28single-precision%29))
  (Rendering|Components|TextRender|SetText (Variables|Default|GetTextRender) (Utilities|Text|ToText(Integer) (Variables|Default|GetCountdownTimer))))

(fn ConstructionScript)

(fn OnRepDeactivate
  (Components|Activation|Deactivate (Variables|Default|GetP_Fire)))